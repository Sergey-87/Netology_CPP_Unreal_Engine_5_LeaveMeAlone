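; Player controller Blueprint for LeaveMeAlone that handles the Pause input action, branching on an OnPause flag.
; When the flag is false, it sets it, creates and shows WBP_Pause, pauses the game and switches to UI-only input with the cursor visible.
; When true, it removes the widget, unpauses and restores game-only input with a hidden cursor, but never clears OnPause itself.
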(event `InputAction|Pause`
  (params (Key :type "Key Structure"))
  (bind _returnvalue (`GameplayStatics.GetPlayerController` 0))
  (bind _returnvalue_2 (`GameplayStatics.GetPlayerController` 0))
  (:`Pressed`
    (if (`self.OnPause`)
      (`Widget.RemoveFromParent` (`self.PauseWidget`))
      (`GameplayStatics.SetGamePaused` false)
      (`WidgetBlueprintLibrary.SetInputMode_GameOnly` _returnvalue)
      (set `PlayerController.bShowMouseCursor` false _returnvalue)
      (else
        (set `self.OnPause` true)
        (bind _returnvalue_3 (`|CreateWidget` "/Game/LeaveMeAlone/Widgets/WBP_Pause.WBP_Pause_C"))
        (bind _output_get (set `self.PauseWidget` _returnvalue_3))
        (`UserWidget.AddToViewport` _output_get 0)
        (`GameplayStatics.SetGamePaused` true)
        (`WidgetBlueprintLibrary.SetInputMode_UIOnlyEx` _returnvalue_2 _output_get)
        (set `PlayerController.bShowMouseCursor` true _returnvalue_2)))))

(fn `UserConstructionScript`)